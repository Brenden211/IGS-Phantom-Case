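; BP_Spawner is an actor that supplies random, non-repeating spawn locations.
; On BeginPlay it caches the world locations of the scene components attached directly under its root as the spawn point pool.
; GetRandomSpawn picks a random location and removes it from the pool, so each point is handed out once.
; When the pool is empty, it prints a warning and returns the zero vector.
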(event `self.ReceiveBeginPlay`
  (for _array_element (`SceneComponent.GetChildrenComponents` (`self.DefaultSceneRoot`) false)
    (`KismetArrayLibrary.Array_Add` (`self.SpawnPoints`) (`SceneComponent.K2_GetComponentLocation` _array_element))))

(fn `GetRandomSpawn`
  (returns (SpawnPoint :type "Vector Structure"))
  (if (> (`KismetArrayLibrary.Array_Length` (`self.SpawnPoints`)) 0)
    (bind _output_get (set `self.RandSpawn` (`KismetMathLibrary.RandomIntegerInRange` 0 (- (`KismetArrayLibrary.Array_Length` (`self.SpawnPoints`)) 1))))
    (set `self.aSpawn` (`|GetArrayItem` (`self.SpawnPoints`) _output_get))
    (`KismetArrayLibrary.Array_Remove` (`self.SpawnPoints`) _output_get)
    (return (`self.aSpawn`))
    (else
      (`KismetSystemLibrary.PrintString` "No Spawn Found" true true (struct :`R` 1.0 :`B` 0.020931 :`A` 1.0))
      (return (0.0 0.0 0.0)))))

(fn `UserConstructionScript`)