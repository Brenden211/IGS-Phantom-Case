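; BP_Player_Flashlight is a flashlight actor that switches a spotlight on and off.
; ToggleLight flips the IsLight flag and sets the SpotLight intensity to either zero or SpotIntensity.
; BeginPlay calls ToggleLight once, so the starting state is the inverse of the IsLight default.
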(event `self.ReceiveBeginPlay`
  (`self.Toggle Light`))

(event `Toggle Light`
  (if (`self.isLight`)
    (set `self.isLight` false)
    (`LightComponent.SetIntensity` (`self.SpotLight`) 0.0)
    (else
      (set `self.isLight` true)
      (`LightComponent.SetIntensity` (`self.SpotLight`) (`self.Spot Intensity`)))))

(fn `UserConstructionScript`)