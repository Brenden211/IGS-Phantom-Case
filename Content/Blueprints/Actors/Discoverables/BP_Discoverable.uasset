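; Discoverable actor that shows an interact icon with configurable text when the first-person character overlaps its collision.
; Interacting passes its info text to the character's Discover and irritates demo ghosts found by a sphere overlap around the mesh.
; A DoOnce blocks repeats until a two-second delay resets it and calls Interacted.
; Overlap begin and end share one FlipFlop visibility toggle; CanInteract always returns false.
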(event `self.ReceiveBeginPlay`
  (bind _aswb_interact_icon (cast `/Game/Dynamic/UI/WB_InteractIcon` (`WidgetComponent.GetWidget` (`self.Widget`))))
  (`/Game/Dynamic/UI/WB_InteractIcon.SetText` _aswb_interact_icon (`self.InteractText`)))

(event `self.Interact`
  (`/Engine/EditorBlueprintResources/StandardMacros.DoOnce` false :!label _label
    (:`Completed`
      (bind _asbp_fp_character (cast `/Game/Blueprints/Character/Player/BP_FP_Character` (`GameplayStatics.GetPlayerCharacter` 0)))
      (`/Game/Blueprints/Character/Player/BP_FP_Character.Discover` _asbp_fp_character (`self.InfoText`))
      (bind _outactors (`KismetSystemLibrary.SphereOverlapActors` (`SceneComponent.K2_GetComponentLocation` (`self.StaticMesh`)) (`self.IrritateRadius`) (`self.OverlapTypes`) "/Game/Blueprints/Character/Enemy/BP_Character_DemoGhost.BP_Character_DemoGhost_C"))
      (for _array_element _outactors
        (bind _asbp_character_demo_ghost (cast `/Game/Blueprints/Character/Enemy/BP_Character_DemoGhost` _array_element))
        (`/Game/Blueprints/Character/Enemy/BP_Character_DemoGhost.Irritate` _asbp_character_demo_ghost (`self.IrritateAmount`)))
      (`KismetSystemLibrary.Delay` 2.0)
      (`self.Reset Interact`)
      (`self.Interacted`))))

(event `Reset Interact`
  (goto _label :!via `Reset`))

(event `self.Interact Collision.OnComponentBeginOverlap`
  (params (OverlappedComponent :type "PrimitiveComponent Object Reference") (OtherActor :type "Actor Object Reference") (OtherComp :type "PrimitiveComponent Object Reference") (OtherBodyIndex :type Integer) (bFromSweep :type Boolean) (SweepResult :type "HitResult Structure (by ref)"))
  (cast `/Game/Blueprints/Character/Player/BP_FP_Character` OtherActor)
  (`self.Toggle Interact Widget`))

(event `self.Interact Collision.OnComponentEndOverlap`
  (params (OverlappedComponent :type "PrimitiveComponent Object Reference") (OtherActor :type "Actor Object Reference") (OtherComp :type "PrimitiveComponent Object Reference") (OtherBodyIndex :type Integer))
  (cast `/Game/Blueprints/Character/Player/BP_FP_Character` OtherActor)
  (`self.Toggle Interact Widget`))

(event `Toggle Interact Widget`
  (bind _isa (`/Engine/EditorBlueprintResources/StandardMacros.FlipFlop`)
    (:`A`
      _)
    (:`B`
      _))
  (`SceneComponent.SetHiddenInGame` (`self.Widget`) (not _isa) false))

(fn `CanInteract`
  (returns (`Output Value` :type Boolean))
  (return false))

(fn `UserConstructionScript`)