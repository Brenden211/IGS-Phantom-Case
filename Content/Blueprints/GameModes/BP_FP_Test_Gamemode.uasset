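; Game mode for a whodunit mystery that randomizes the guilty person, weapon and room, then checks the player's guess in Solve.
; On BeginPlay it draws unique room-weapon-person sets, making the first the truth.
; Sets spawn an item and hint whispers, innocent ones add exonerating major whispers, and one random set gets only an ambiguous room clue instead of an item.
; A separate clue-score win/lose flow remains, its list setup disconnected.
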(event `self.ReceiveBeginPlay`
  (bind _outactors (`GameplayStatics.GetAllActorsOfClass` "/Game/Blueprints/Actors/BP_Room.BP_Room_C"))
  (set `self.Rooms` _outactors)
  (bind _returnvalue (`GameplayStatics.GetActorOfClass` "/Game/Blueprints/Actors/BP_Spawner.BP_Spawner_C"))
  (set `self.WhisperSpawner` _returnvalue)
  (`self.InitializeEvidence`))

(event `Get All Clue Actors`
  (bind _outactors (`GameplayStatics.GetAllActorsOfClass` "/Game/Blueprints/Actors/PastClues/BP_Clue.BP_Clue_C"))
  (bind _output_get (set `self.Temp Clue Actor List` _outactors))
  (set `self.Sorted Clue Actor List` _output_get))

(event `Sort Clue Actor List by Name`)

(event `Set Clue Bool List`
  (for (_array_element _array_index) (`self.Sorted Clue Actor List`)
    (`KismetArrayLibrary.Array_Set` (`self.Clue Importance List`) _array_index (`/Game/Blueprints/Actors/PastClues/BP_Clue.isImportant` _array_element))))

(event `Set Game State`
  (params (`Input Clue List` :type "Array of Boolean"))
  (set `self.PlayerClueScore` 0)
  (for (_array_element _array_index) `Input Clue List`
    (`KismetSystemLibrary.PrintString` (`KismetStringLibrary.Conv_BoolToString` _array_element))
    (if (== _array_element (`|GetArrayItem` (`self.Clue Importance List`) _array_index))
      (`/Engine/EditorBlueprintResources/StandardMacros.IncrementInt` (`self.PlayerClueScore`))))
  (`self.Check Game State`)
  (`KismetSystemLibrary.PrintString` (`KismetStringLibrary.Conv_IntToString` (`self.PlayerClueScore`))))

(event `Check Game State`
  (bind _returnvalue (`GameplayStatics.GetPlayerController` 0))
  (if (== (`self.PlayerClueScore`) (`self.ClueScore`))
    (bind _returnvalue_2 (`|CreateWidget` "/Game/Dynamic/UI/WB_GameWonPrompt.WB_GameWonPrompt_C" _returnvalue))
    (`UserWidget.AddToViewport` _returnvalue_2 0)
    (`KismetSystemLibrary.Delay` 3.0)
    (`Widget.RemoveFromParent` _returnvalue_2)
    (else
      (bind _returnvalue_3 (`|CreateWidget` "/Game/Dynamic/UI/WB_GameLostPrompt.WB_GameLostPrompt_C" _returnvalue))
      (`UserWidget.AddToViewport` _returnvalue_3 0)
      (`KismetSystemLibrary.Delay` 3.0)
      (`Widget.RemoveFromParent` _returnvalue_3))))

(fn `AmbigousRoomClue`
  (if (== (`KismetMathLibrary.RandomIntegerInRange` 0 1) 0)
    (set `self.EvidenceText` (`KismetStringLibrary.Concat_StrStr` "A Weapon" " Was in " (`|GetEnumeratorNameAsString` (`self.CurRoomType`))))
    (else
      (set `self.EvidenceText` (`KismetStringLibrary.Concat_StrStr` "Someone" " Was in " (`|GetEnumeratorNameAsString` (`self.CurRoomType`))))))
  (bind _spawnpoint (`/Game/Blueprints/Actors/BP_Spawner.GetRandomSpawn` (`self.WhisperSpawner`)))
  (bind _returnvalue (`|SpawnActorFromClass` "/Game/Blueprints/Actors/Discoverables/BP_Whisper.BP_Whisper_C" (`KismetMathLibrary.Conv_VectorToTransform` _spawnpoint) "Undefined" "MultiplyWithRoot" null null))
  (set `/Game/Blueprints/Actors/Discoverables/BP_Discoverable.InfoText` (`self.EvidenceText`) _returnvalue))

(fn `Choose Set`
  ;[1 1 1] Get Random Room and Remove From List
  (bind _output_get (set `self.RandInt` (`KismetMathLibrary.RandomIntegerInRange` 0 (- (`KismetArrayLibrary.Array_Length` (`self.Rooms`)) 1))))
  (set `self.CurRoom` (`|GetArrayItem` (`self.Rooms`) _output_get))
  (`KismetArrayLibrary.Array_Remove` (`self.Rooms`) (`self.RandInt`))
  ;[1 1 1] Get Random Weapon and Remove From List
  (bind _output_get_2 (set `self.RandInt` (`KismetMathLibrary.RandomIntegerInRange` 0 (- (`KismetArrayLibrary.Array_Length` (`self.Weapons`)) 1))))
  (set `self.CurWeapon` (`|GetArrayItem` (`self.Weapons`) _output_get_2))
  (`KismetArrayLibrary.Array_Remove` (`self.Weapons`) (`self.RandInt`))
  ;[1 1 1] Get Random Person and Remove From List
  (bind _output_get_3 (set `self.RandInt` (`KismetMathLibrary.RandomIntegerInRange` 0 (- (`KismetArrayLibrary.Array_Length` (`self.People`)) 1))))
  (set `self.CurPerson` (`|GetArrayItem` (`self.People`) _output_get_3))
  (`KismetArrayLibrary.Array_Remove` (`self.People`) (`self.RandInt`))
  ;[1 1 1] Retrieve Types
  (bind _output_get_4 (set `self.CurRoomType` (`/Game/Blueprints/Actors/BP_Room.RoomType` (`self.CurRoom`))))
  (bind _type (`self.WeaponClassToType` (`self.CurWeapon`)))
  (bind _output_get_5 (set `self.CurWeaponType` _type))
  (bind _type_2 (`self.PersonClassToType` (`self.CurPerson`)))
  (bind _output_get_6 (set `self.CurPersonType` _type_2)))

(fn `GetTruthText`
  (returns (Solution :type String))
  (return (`KismetStringLibrary.Concat_StrStr` "" (`|GetEnumeratorNameAsString` (`self.TruePerson`)) " in " (`|GetEnumeratorNameAsString` (`self.TrueRoom`)) " With The " (`|GetEnumeratorNameAsString` (`self.TrueWeapon`)))))

(fn `InitializeEvidence`
  (bind _output_get (set `self.EvidenceCount` (- (`KismetMathLibrary.Min` (`KismetArrayLibrary.Array_Length` (`self.Rooms`)) (`KismetArrayLibrary.Array_Length` (`self.Weapons`)) (`KismetArrayLibrary.Array_Length` (`self.People`))) 1)))
  (if (!= _output_get -1)
    (set `self.RandRemove` (`KismetMathLibrary.RandomIntegerInRange` 0 (`self.EvidenceCount`)))
    (`self.Choose Set`)
    (set `self.TrueRoom` (`self.CurRoomType`))
    (set `self.TrueWeapon` (`self.CurWeaponType`))
    (set `self.TruePerson` (`self.CurPersonType`))
    (if (== 0 (`self.RandRemove`))
      (`self.AmbigousRoomClue`)
      (else
        (`self.SetDiscoverables` false)))
    (for _index (range 1 (+ (`self.EvidenceCount`) 1))
      (`self.Choose Set`)
      (if (== _index (`self.RandRemove`))
        (`self.SpawnMajorEvidence`)
        (`self.AmbigousRoomClue`)
        (else
          (`self.SetDiscoverables` true))))
    (else
      (`KismetSystemLibrary.PrintString` "Cannot Initialize Evidence"))))

(fn `PersonClassToType`
  (params (Class :type "/Game/Blueprints/Actors/Discoverables/BP_Person Class Reference"))
  (returns (Type :type "/Game/Blueprints/Enums/E_People Enum"))
  (castclass `/Game/Blueprints/Actors/Discoverables/BP_Person_SallyPurse` Class
    (:`then`
      (return "NewEnumerator0"))
    (:`CastFailed`
      (castclass `/Game/Blueprints/Actors/Discoverables/BP_Person_JohnCoat` Class
        (:`then`
          (return "NewEnumerator1"))
        (:`CastFailed`
          (castclass `/Game/Blueprints/Actors/Discoverables/BP_Person_AlexPhone` Class
            (:`then`
              (return "NewEnumerator2"))
            (:`CastFailed`
              (castclass `/Game/Blueprints/Actors/Discoverables/BP_Person_LillyLetter` Class
                (:`then`
                  (return "NewEnumerator3"))
                (:`CastFailed`
                  (castclass `/Game/Blueprints/Actors/Discoverables/BP_Person_GeorgeHat` Class)
                  (return "NewEnumerator4"))))))))))

(fn `SetDiscoverables`
  (params (Innocent :type Boolean))
  ;[1 1 1] Choose Which Clue To Show
  (if (== (`KismetMathLibrary.RandomIntegerInRange` 0 1) 0)
    (bind _spawnpoint (`/Game/Blueprints/Actors/BP_Spawner.GetRandomSpawn` (`self.CurRoom`)))
    (`|SpawnActorFromClass` (`self.CurWeapon`) (`KismetMathLibrary.Conv_VectorToTransform` _spawnpoint) "Undefined" "MultiplyWithRoot" null null)
    (`self.SpawnMinorEvidence` false)
    (else
      (bind _spawnpoint_2 (`/Game/Blueprints/Actors/BP_Spawner.GetRandomSpawn` (`self.CurRoom`)))
      (`|SpawnActorFromClass` (`self.CurPerson`) (`KismetMathLibrary.Conv_VectorToTransform` _spawnpoint_2) "Undefined" "MultiplyWithRoot" null null)
      (`self.SpawnMinorEvidence` true)))
  (if Innocent
    (`self.SpawnMajorEvidence`)))

(fn `Solve`
  (params (Room :type "/Game/Blueprints/Enums/E_Room Enum" :default "NewEnumerator0") (Weapon :type "/Game/Blueprints/Enums/E_Weapon Enum" :default "NewEnumerator0") (Person :type "/Game/Blueprints/Enums/E_People Enum" :default "NewEnumerator0"))
  (set `self.Solved` (and (`|EnumEquality` Room (`self.TrueRoom`)) (`|EnumEquality` Weapon (`self.TrueWeapon`)) (`|EnumEquality` Person (`self.TruePerson`))))
  (bind _returnvalue (`|CreateWidget` "/Game/Dynamic/UI/BlurToWidget.BlurToWidget_C"))
  (`/Game/Dynamic/UI/BlurToWidget.BlurOpenWidget` _returnvalue "/Game/Dynamic/UI/SolveWidget.SolveWidget_C"))

(fn `SpawnMajorEvidence`
  (switch `int` (`KismetMathLibrary.RandomIntegerInRange` 0 2)
    (:`0`
      (`self.SpawnRoomEvidence` (`self.CurRoomType`)))
    (:`1`
      (switch `/Game/Blueprints/Enums/E_Weapon` (`self.CurWeaponType`)
        (:`NewEnumerator0`
          (set `self.EvidenceText` "The Knife is Clean"))
        (:`NewEnumerator1`
          (set `self.EvidenceText` "The Gun is Unfired"))
        (:`NewEnumerator2`
          (set `self.EvidenceText` "The Laptop is Undamaged"))
        (:`NewEnumerator3`
          (set `self.EvidenceText` "The Rope is Untouched"))
        (:`NewEnumerator4`
          (set `self.EvidenceText` "The Statue is Unmoved")))
      (bind _spawnpoint (`/Game/Blueprints/Actors/BP_Spawner.GetRandomSpawn` (`self.WhisperSpawner`) :!label _label))
      (bind _returnvalue (`|SpawnActorFromClass` "/Game/Blueprints/Actors/Discoverables/BP_Major_Whisper.BP_Major_Whisper_C" (`KismetMathLibrary.Conv_VectorToTransform` _spawnpoint) "Undefined" "MultiplyWithRoot" null null))
      (set `/Game/Blueprints/Actors/Discoverables/BP_Discoverable.InfoText` (`self.EvidenceText`) _returnvalue))
    (:`2`
      (switch `/Game/Blueprints/Enums/E_People` (`self.CurPersonType`)
        (:`NewEnumerator0`
          (set `self.EvidenceText` "Sally Wouldn't Hurt a Fly")
          (goto _label))
        (:`NewEnumerator1`
          (set `self.EvidenceText` "John Played No Part in This")
          (goto _label))
        (:`NewEnumerator2`
          (set `self.EvidenceText` "Alex Couldn't Have Done This")
          (goto _label))
        (:`NewEnumerator3`
          (set `self.EvidenceText` "Lilly Did Nothing Wrong")
          (goto _label))
        (:`NewEnumerator4`
          (set `self.EvidenceText` "George Was Fast Asleep")
          (goto _label))))))

(fn `SpawnMinorEvidence`
  (params (ForWeapon :type Boolean))
  (if ForWeapon
    (if (== (`KismetMathLibrary.RandomIntegerInRange` 0 1) 0)
      (set `self.EvidenceText` (`KismetStringLibrary.Concat_StrStr` "The " (`|GetEnumeratorNameAsString` (`self.CurWeaponType`)) " Was in " (`|GetEnumeratorNameAsString` (`self.CurRoomType`))))
      (else
        (set `self.EvidenceText` (`KismetStringLibrary.Concat_StrStr` (`|GetEnumeratorNameAsString` (`self.CurPersonType`)) " Had The " (`|GetEnumeratorNameAsString` (`self.CurWeaponType`))) :!label _label)))
    (elif (== (`KismetMathLibrary.RandomIntegerInRange` 0 1) 0)
      (goto _label)
      (else
        (set `self.EvidenceText` (`KismetStringLibrary.Concat_StrStr` (`|GetEnumeratorNameAsString` (`self.CurPersonType`)) " Was in " (`|GetEnumeratorNameAsString` (`self.CurRoomType`)))))))
  (bind _spawnpoint (`/Game/Blueprints/Actors/BP_Spawner.GetRandomSpawn` (`self.WhisperSpawner`)))
  (bind _returnvalue (`|SpawnActorFromClass` "/Game/Blueprints/Actors/Discoverables/BP_Whisper.BP_Whisper_C" (`KismetMathLibrary.Conv_VectorToTransform` _spawnpoint) "Undefined" "MultiplyWithRoot" null null))
  (set `/Game/Blueprints/Actors/Discoverables/BP_Discoverable.InfoText` (`self.EvidenceText`) _returnvalue))

(fn `SpawnRoomEvidence`
  (params (Room :type "/Game/Blueprints/Enums/E_Room Enum" :default "NewEnumerator0"))
  (switch `/Game/Blueprints/Enums/E_Room` Room
    (:`NewEnumerator0`
      (set `self.EvidenceText` "Your Bedroom is Undisturbed"))
    (:`NewEnumerator1`
      (set `self.EvidenceText` "The Bathroom is Clean"))
    (:`NewEnumerator2`
      (set `self.EvidenceText` "The Kitchen is Spotless"))
    (:`NewEnumerator3`
      (set `self.EvidenceText` "The Dining Room is Pristine"))
    (:`NewEnumerator4`
      (set `self.EvidenceText` "The Living Room is Untouched"))
    (:`NewEnumerator6`
      (set `self.EvidenceText` "The Master Bedroom is Tidy"))
    (:`NewEnumerator7`
      (set `self.EvidenceText` "The Spare Bedroom Gathers Dust"))
    (:`NewEnumerator8`
      (set `self.EvidenceText` "The Upstairs Bathroom Shines"))
    (:`NewEnumerator9`
      (set `self.EvidenceText` "The Office is Organized")))
  (bind _spawnpoint (`/Game/Blueprints/Actors/BP_Spawner.GetRandomSpawn` (`self.WhisperSpawner`)))
  (bind _returnvalue (`|SpawnActorFromClass` "/Game/Blueprints/Actors/Discoverables/BP_Major_Whisper.BP_Major_Whisper_C" (`KismetMathLibrary.Conv_VectorToTransform` _spawnpoint) "Undefined" "MultiplyWithRoot" null null))
  (set `/Game/Blueprints/Actors/Discoverables/BP_Discoverable.InfoText` (`self.EvidenceText`) _returnvalue))

(fn `UserConstructionScript`)

(fn `WeaponClassToType`
  (params (Class :type "/Game/Blueprints/Actors/Discoverables/BP_Weapon Class Reference"))
  (returns (Type :type "/Game/Blueprints/Enums/E_Weapon Enum"))
  (castclass `/Game/Blueprints/Actors/Discoverables/BP_Weapon_Knife` Class
    (:`then`
      (return "NewEnumerator0"))
    (:`CastFailed`
      (castclass `/Game/Blueprints/Actors/Discoverables/BP_Weapon_Gun` Class
        (:`then`
          (return "NewEnumerator1"))
        (:`CastFailed`
          (castclass `/Game/Blueprints/Actors/Discoverables/BP_Weapon_Laptop` Class
            (:`then`
              (return "NewEnumerator2"))
            (:`CastFailed`
              (castclass `/Game/Blueprints/Actors/Discoverables/BP_Weapon_Rope` Class
                (:`then`
                  (return "NewEnumerator3"))
                (:`CastFailed`
                  (castclass `/Game/Blueprints/Actors/Discoverables/BP_Weapon_Statue` Class)
                  (return "NewEnumerator4"))))))))))