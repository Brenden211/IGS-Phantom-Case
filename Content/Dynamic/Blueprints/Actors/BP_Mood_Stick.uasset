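; BP_Mood_Stick is an actor whose stick material and light take on the mood color of the nearest demo ghost inside its detection volume.
; Overlap events maintain the list of close ghosts, and a countdown on Tick periodically runs GetColor to pick the closest one, falling back to white when none are near.
; When the target color changes, Tick blends the dynamic material and light from the current color to it over LerpTime.
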(event `self.ReceiveBeginPlay`
  (bind _returnvalue (`PrimitiveComponent.CreateDynamicMaterialInstance` (`self.ColorStick`) 0 null "None"))
  (bind _output_get (set `self.dynamicMaterial` _returnvalue))
  (`MaterialInstanceDynamic.SetVectorParameterValue` _output_get "color" (struct :`R` 1.0 :`G` 1.0 :`B` 1.0 :`A` 1.0)))

(event `self.Detection.OnComponentBeginOverlap`
  (params (OverlappedComponent :type "PrimitiveComponent Object Reference") (OtherActor :type "Actor Object Reference") (OtherComp :type "PrimitiveComponent Object Reference") (OtherBodyIndex :type Integer) (bFromSweep :type Boolean) (SweepResult :type "HitResult Structure (by ref)"))
  (bind _asbp_character_demo_ghost (cast `/Game/Dynamic/Blueprints/Character/Enemy/BP_Character_DemoGhost` OtherActor))
  (`KismetArrayLibrary.Array_Add` (`self.CloseGhosts`) _asbp_character_demo_ghost))

(event `self.Detection.OnComponentEndOverlap`
  (params (OverlappedComponent :type "PrimitiveComponent Object Reference") (OtherActor :type "Actor Object Reference") (OtherComp :type "PrimitiveComponent Object Reference") (OtherBodyIndex :type Integer))
  (bind _asbp_character_demo_ghost (cast `/Game/Dynamic/Blueprints/Character/Enemy/BP_Character_DemoGhost` OtherActor))
  (`KismetArrayLibrary.Array_RemoveItem` (`self.CloseGhosts`) _asbp_character_demo_ghost))

(event `self.ReceiveTick`
  (params (DeltaSeconds :type "Float (single-precision)"))
  (bind _moodcolor (`self.MoodColor`))
  (bind _returnvalue (`KismetMathLibrary.LinearColorLerp` (`self.MoodColor`) (`self.currentColor`) (/ (`self.lerping`) (`self.LerpTime`))))
  (bind _output_get (set `self.NextCheck` (- (`self.NextCheck`) DeltaSeconds)))
  (if (<= _output_get 0.0)
    (`self.GetColor`)
    (set `self.NextCheck` (`self.CheckTimer`)))
  (if (> (`self.lerping`) 0.0)
    (bind _output_get_2 (set `self.lerping` (- (`self.lerping`) DeltaSeconds)))
    (if (<= _output_get_2 0.0)
      (`MaterialInstanceDynamic.SetVectorParameterValue` (`self.dynamicMaterial`) "color" _moodcolor)
      (`LightComponent.SetLightColor` (`self.ColorLight`) _moodcolor true)
      (else
        (`MaterialInstanceDynamic.SetVectorParameterValue` (`self.dynamicMaterial`) "color" _returnvalue)
        (`LightComponent.SetLightColor` (`self.ColorLight`) _returnvalue true)))))

(fn `GetColor`
  (bind _output (`|GetArrayItem` (`self.CloseGhosts`)))
  (if (== (`KismetArrayLibrary.Array_Length` (`self.CloseGhosts`)) 0)
    (if (!= (`self.MoodColor`) (struct :`R` 1.0 :`G` 1.0 :`B` 1.0 :`A` 1.0))
      (set `self.MoodColor` (struct :`R` 1.0 :`G` 1.0 :`B` 1.0 :`A` 1.0))
      (bind _returnvalue (`MaterialInstanceDynamic.K2_GetVectorParameterValue` (`self.dynamicMaterial`) "color" :!label _label))
      (set `self.currentColor` _returnvalue)
      (set `self.lerping` (`self.LerpTime`)))
    (else
      (set `self.minGhost` _output)
      (set `self.minDist` (`self.GetDistanceTo` _output))
      (for _array_element (`self.CloseGhosts`)
        (bind _returnvalue_2 (`self.GetDistanceTo` _array_element))
        (if (< _returnvalue_2 (`self.minDist`))
          (set `self.minDist` _returnvalue_2)
          (set `self.minGhost` _array_element)))
      (bind _moodcolor (`/Game/Dynamic/Blueprints/Character/Enemy/BP_Character_DemoGhost.GetMoodColor` (`self.minGhost`)))
      (if (!= (`self.MoodColor`) _moodcolor)
        (set `self.MoodColor` _moodcolor)
        (goto _label)))))

(fn `UserConstructionScript`)