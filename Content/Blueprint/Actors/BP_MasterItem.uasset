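; BP_MasterItem is an interactable item actor, apparently a base for items, that signals to the first-person player when it can be used.
; Sphere overlap with CH_FP_Player, gated by CanInteract, creates or removes a WB_InteractText prompt in the widget component and toggles an outline overlay material and CanPressKey.
; The CanReceiveTrace event also toggles the outline and CanPressKey while the prompt exists, leaving the interaction itself outside this graph.
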(event `self.Sphere.OnComponentBeginOverlap`
  (params (OverlappedComponent :type "PrimitiveComponent Object Reference") (OtherActor :type "Actor Object Reference") (OtherComp :type "PrimitiveComponent Object Reference") (OtherBodyIndex :type Integer) (bFromSweep :type Boolean) (SweepResult :type "HitResult Structure (by ref)"))
  (bind _widget (`self.Widget`))
  (cast `/Game/Blueprint/Character/Player/CH_FP_Player` OtherActor)
  (if (`self.CanInteract`)
    (bind _returnvalue (`|CreateWidget` "/Game/UI/WB_InteractText.WB_InteractText_C" (`GameplayStatics.GetPlayerController` 0)))
    (bind _output_get (set `self.InteractionWidget` _returnvalue))
    (`WidgetComponent.SetWidget` _widget _output_get)
    (`SceneComponent.SetVisibility` _widget true false)
    (`self.InteractionWidget`
      (:`then`
        (`MeshComponent.SetOverlayMaterial` (`self.StaticMesh`) "/Game/Material/M_Outline.M_Outline")
        (set `self.CanPressKey` true))
      (:`else`))))

(event `self.Sphere.OnComponentEndOverlap`
  (params (OverlappedComponent :type "PrimitiveComponent Object Reference") (OtherActor :type "Actor Object Reference") (OtherComp :type "PrimitiveComponent Object Reference") (OtherBodyIndex :type Integer))
  (cast `/Game/Blueprint/Character/Player/CH_FP_Player` OtherActor)
  (if (`self.CanInteract`)
    (`self.InteractionWidget`
      (:`then`
        (set `self.CanPressKey` false)
        (`MeshComponent.SetOverlayMaterial` (`self.StaticMesh`) null)
        (`Widget.RemoveFromParent` (`self.InteractionWidget`))
        (set `self.InteractionWidget` null)
        (`SceneComponent.SetVisibility` (`self.Widget`) false false))
      (:`else`))))

(event `/Game/Blueprint/Interface/BPI_Interactable.Can Receive Trace`
  (params (`Can Interact` :type Boolean))
  (if (`self.CanInteract`)
    (if `Can Interact`
      (`self.InteractionWidget`
        (:`then`
          (`MeshComponent.SetOverlayMaterial` (`self.StaticMesh`) "/Game/Material/M_Outline.M_Outline")
          (set `self.CanPressKey` true))
        (:`else`)))
    (else
      (`self.InteractionWidget`
        (:`then`
          (`MeshComponent.SetOverlayMaterial` (`self.StaticMesh`) null)
          (set `self.CanPressKey` false))
        (:`else`)))))

(fn `UserConstructionScript`)