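; Demo ghost enemy whose mood governs whether it patrols or hunts the player.
; Touches and Irritate calls change mood, which decays over time; above AngryThreshold, sighting starts a chase and contact kills the player, removing the ghost.
; TransitionTo idles before switching state and tuning movement, while UpdateBB feeds the AI Blackboard.
; Tick bobs the mesh and switches to investigating the player's last position after TimeToLost without a sighting.
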(event `self.ReceiveBeginPlay`
  (bind _returnvalue (`AIBlueprintHelperLibrary.GetBlackboard` (`AIBlueprintHelperLibrary.GetAIController` self)))
  (`KismetSystemLibrary.Delay` 0.2)
  (`/Engine/EditorBlueprintResources/StandardMacros.IsValid` _returnvalue
    (:`Is Valid`
      (set `self.Blackboard` _returnvalue)
      (set `self.CurrentMood` (`KismetMathLibrary.RandomIntegerInRange` 40 60))
      (bind _output_get (set `self.MoodDropRate` (`KismetMathLibrary.RandomFloatInRange` 10.0 20.0)))
      (set `self.NextMoodDrop` _output_get)
      (bind _output_get_2 (set `self.CurrentState` "NewEnumerator1"))
      (`self.UpdateBB` _output_get_2))))

(event `self.PawnSensing.OnSeePawn`
  (params (Pawn :type "Pawn Object Reference"))
  (if (and (> (`self.CurrentMood`) (`self.AngryThreshold`)) (not (`self.WaitingToAnger`)))
    (bind _asch_fp_ghost (cast `/Game/Blueprint/Character/Player/CH_FP_Player` Pawn))
    (set `self.SensedPawn` _asch_fp_ghost)
    (set `self.LastSeen` 0.0)
    (`GameplayStatics.PlaySoundAtLocation` "/Game/Static/Audio/SC_Ghost_Alert.SC_Ghost_Alert" (`self.K2_GetActorLocation`) (struct) 1.0 1.0 0.0 null null null null)
    (switch `/Game/Blueprint/Enum/E_Enemy_State` (`self.CurrentState`)
      (:`NewEnumerator1`
        (`self.TransitionTo` 1.0 "NewEnumerator2"))
      (:`NewEnumerator4`
        (`self.TransitionTo` 0.0 "NewEnumerator2")))))

(event `self.ReceiveTick`
  (params (DeltaSeconds :type "Float (single-precision)"))
  (bind _charactermovement (`self.CharacterMovement`))
  (`self.Bob` DeltaSeconds)
  (bind _output_get (set `self.NextMoodDrop` (- (`self.NextMoodDrop`) DeltaSeconds)))
  (if (< _output_get 0.0)
    (set `self.NextMoodDrop` (`self.MoodDropRate`))
    (bind _result (`/Engine/EditorBlueprintResources/StandardMacros.DecrementInt` (`self.CurrentMood`))
      (:`  `
        (if (<= _result (`self.AngryThreshold`))
          (bind _output_get_2 (set `self.CurrentState` "NewEnumerator1"))
          (`self.UpdateBB` _output_get_2)
          (set `CharacterMovementComponent.BrakingDecelerationWalking` 548.0 _charactermovement)
          (set `CharacterMovementComponent.MaxAcceleration` 1048.0 _charactermovement)))))
  (if (`KismetSystemLibrary.IsValid` (`self.SensedPawn`))
    (bind _output_get_3 (set `self.LastSeen` (+ DeltaSeconds (`self.LastSeen`))))
    (if (>= _output_get_3 (`self.TimeToLost`))
      (set `self.LastPos` (`self.K2_GetActorLocation` (`self.SensedPawn`)))
      (set `self.SensedPawn` null)
      (bind _output_get_4 (set `self.CurrentState` "NewEnumerator4"))
      (`self.UpdateBB` _output_get_4))))

(event `Renable Hit`
  (set `self.HitPlayer` false))

(event `self.CapsuleComponent.OnComponentHit`
  (params (HitComponent :type "PrimitiveComponent Object Reference") (OtherActor :type "Actor Object Reference") (OtherComp :type "PrimitiveComponent Object Reference") (NormalImpulse :type "Vector Structure") (Hit :type "HitResult Structure (by ref)"))
  (if (not (`self.HitPlayer`))
    (bind _asch_fp_ghost (cast `/Game/Blueprint/Character/Player/CH_FP_Player` OtherActor))
    (set `self.HitPlayer` true)
    (if (> (`self.CurrentMood`) (`self.AngryThreshold`))
      (set `self.HitPlayer` true)
      (bind _returnvalue (`|CreateWidget` "/Game/UI/BlurToWidget.BlurToWidget_C"))
      (`/Game/UI/BlurToWidget.BlurOpenWidget` _returnvalue "/Game/UI/PlayerDeathWidget.PlayerDeathWidget_C")
      (`self.K2_DestroyActor` _asch_fp_ghost)
      (`self.K2_DestroyActor`)
      (`GameplayStatics.PlaySoundAtLocation` "/Game/Sound/Death.Death" (`self.K2_GetActorLocation`) (struct) 1.0 1.0 0.0 null null null null)
      (else
        (`GameplayStatics.PlaySoundAtLocation` "/Game/Sound/SC_Irritate.SC_Irritate" (`self.K2_GetActorLocation`) (struct) 1.0 1.0 0.0 null null null null)
        (set `self.CurrentMood` (+ (`self.CurrentMood`) (`self.TouchIncrease`)))
        (if (> (`self.CurrentMood`) (`self.AngryThreshold`))
          (set `self.SensedPawn` _asch_fp_ghost)
          (`self.TransitionTo` 2.0 "NewEnumerator2")
          (set `self.LastSeen` 0.0)
          (else
            (`self.TransitionTo` 2.0 "NewEnumerator1")))
        (`KismetSystemLibrary.Delay` 2.0)
        (`self.Renable Hit`)))))

(event `TransitionTo`
  (params (Delay :type "Float (double-precision)") (State :type "/Game/Blueprint/Enum/E_Enemy_State Enum" :default "NewEnumerator0"))
  (bind _charactermovement (`self.CharacterMovement`))
  (bind _charactermovement_2 (`self.CharacterMovement`))
  (bind _output_get (set `self.CurrentState` "NewEnumerator0"))
  (`self.UpdateBB` _output_get)
  ;[1 1 1] Play Animation
  (switch `/Game/Blueprint/Enum/E_Enemy_State` State
    (:`NewEnumerator1`
      (set `self.switchIrritate` false)
      (set `CharacterMovementComponent.BrakingDecelerationWalking` 548.0 _charactermovement)
      (set `CharacterMovementComponent.MaxAcceleration` 1048.0 _charactermovement))
    (:`NewEnumerator4`
      _)
    (:`NewEnumerator2`
      (set `self.switchAngry` true)
      (set `self.WaitingToAnger` true)
      (`GameplayStatics.PlaySoundAtLocation` "/Game/Sound/SC_Angry.SC_Angry" (`self.K2_GetActorLocation`) (struct) 1.0 1.0 0.0 null null null null)))
  (`KismetSystemLibrary.Delay` Delay)
  (set `self.switchAngry` false)
  (set `self.switchIrritate` false)
  (set `self.WaitingToAnger` false)
  (bind _output_get_2 (set `self.CurrentState` State))
  (`self.UpdateBB` _output_get_2)
  (switch `/Game/Blueprint/Enum/E_Enemy_State` State
    (:`NewEnumerator2`
      (`KismetSystemLibrary.Delay` 0.5)
      (set `CharacterMovementComponent.BrakingDecelerationWalking` 0.0 _charactermovement_2)
      (set `CharacterMovementComponent.MaxAcceleration` 5000.0 _charactermovement_2))))

(fn `Bob`
  (params (DeltaTime :type "Float (double-precision)"))
  (`SceneComponent.K2_SetRelativeLocation` (`self.Mesh`) (`KismetMathLibrary.MakeVector` (.x (`SceneComponent.RelativeLocation` (`self.Mesh`))) (.y (`SceneComponent.RelativeLocation` (`self.Mesh`))) (`KismetMathLibrary.Lerp` (`self.StartHeight`) (`self.TopHeight`) (/ (`self.RiseAmount`) (`self.RiseTime`)))) false false)
  (if (`self.Rising`)
    (set `self.RiseAmount` (+ DeltaTime (`self.RiseAmount`)))
    (if (> (`self.RiseAmount`) (`self.RiseTime`))
      (set `self.Rising` false))
    (else
      (set `self.RiseAmount` (- (`self.RiseAmount`) DeltaTime))
      (if (< (`self.RiseAmount`) 0.0)
        (set `self.Rising` true)))))

(fn `GetMoodColor`
  (returns (MoodColor :type "LinearColor Structure"))
  (return (`KismetMathLibrary.SelectColor` (struct :`R` 1.0 :`B` 0.002705 :`A` 1.0) (`KismetMathLibrary.SelectColor` (struct :`R` 0.005482 :`G` 1.0 :`A` 1.0) (struct :`R` 1.0 :`G` 0.789765 :`A` 1.0) (< (`self.CurrentMood`) 25)) (> (`self.CurrentMood`) 50))))

(fn `Irritate`
  (params (Amount :type Integer))
  (`GameplayStatics.PlaySoundAtLocation` "/Game/Sound/SC_Irritate.SC_Irritate" (`self.K2_GetActorLocation`) (struct) 1.0 1.0 0.0 null null null null)
  (bind _output_get (set `self.CurrentMood` (+ (`self.CurrentMood`) Amount)))
  (if (< _output_get 0)
    (set `self.CurrentMood` Amount)
    (elif (> (`self.CurrentMood`) (`self.AngryThreshold`))
      (set `self.SensedPawn` (`GameplayStatics.GetPlayerPawn` 0))
      (set `self.LastSeen` -1.0)
      (switch `/Game/Blueprint/Enum/E_Enemy_State` (`self.CurrentState`)
        (:`NewEnumerator1`
          (`self.TransitionTo` 1.0 "NewEnumerator2")))
      (else
        (`self.TransitionTo` 1.0 "NewEnumerator1")))))

(fn `UpdateBB`
  (params (State :type "/Game/Blueprint/Enum/E_Enemy_State Enum" :default "NewEnumerator0"))
  (`BlackboardComponent.SetValueAsEnum` (`self.Blackboard`) "CurrentState" State)
  (`BlackboardComponent.SetValueAsVector` (`self.Blackboard`) "LastPos" (`self.LastPos`))
  (`BlackboardComponent.SetValueAsObject` (`self.Blackboard`) "Player" (`self.SensedPawn`))
  (`BlackboardComponent.SetValueAsInt` (`self.Blackboard`) "Mood" (`self.CurrentMood`)))

(fn `UserConstructionScript`)